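; Player controller Blueprint that shows the mouse cursor and enables click events when play begins.
; A right mouse button input stores the cursor position and hides the cursor while held, then restores that position and shows the cursor on release.
; An author note marks this cursor-hiding behavior as broken.
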(event `self.ReceiveBeginPlay`
  (set `self.bShowMouseCursor` true)
  (set `self.bEnableClickEvents` true))

(event `Key|Ctrl+Alt+Shift+RightMouseButton`
  (params (Key :type "Key Structure"))
  (bind (_mouseposition_x _mouseposition_y) (`KismetMathLibrary.BreakVector` (`self.mousePosition`)))
  (bind (_locationx _locationy) (`self.GetMousePosition` (`GameplayStatics.GetPlayerController` 0)))
  (:`Pressed`
    (set `self.mousePosition` (`KismetMathLibrary.MakeVector` _locationx _locationy))
    (set `self.bShowMouseCursor` false))
  (:`Released`
    (`self.SetMouseLocation` (`KismetMathLibrary.FTrunc` _mouseposition_x) (`KismetMathLibrary.FTrunc` _mouseposition_y))
    (set `self.bShowMouseCursor` true)))

(fn `UserConstructionScript`)