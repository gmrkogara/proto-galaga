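; Player pawn or character Blueprint that handles keyboard movement and yaw turning.
; W/S and A/D key events set forward and strafe scale variables, and releasing either key of a pair zeroes that axis.
; Every Tick, DoMove feeds those scales into AddMovementInput along the actor's forward and right vectors, then adds controller yaw from an input axis value.
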(event `self.ReceiveTick`
  (params (DeltaSeconds :type "Float (single-precision)"))
  (`self.DoMove`))

(event `DoMove`
  ;[1 1 1] do move
  (`self.AddMovementInput` (`self.GetActorForwardVector`) (`self.moveScaleX`))
  (`self.AddMovementInput` (`self.GetActorRightVector`) (`self.moveScaleY`))
  (`self.AddControllerYawInput` (`self.GetInputAxisKeyValue`)))

(event `Key|W`
  (params (Key :type "Key Structure"))
  ;[1 1 1] move updown keys
  (:`Pressed`
    (set `self.moveScaleX` 1.0))
  (:`Released`
    (set `self.moveScaleX` 0.0 :!label _label)))

(event `Key|A`
  (params (Key :type "Key Structure"))
  ;[1 1 1] move left right keys
  (:`Pressed`
    (set `self.moveScaleY` -1.0))
  (:`Released`
    (set `self.moveScaleY` 0.0 :!label _label_2)))

(event `Key|S`
  (params (Key :type "Key Structure"))
  ;[1 1 1] move updown keys
  (:`Pressed`
    (set `self.moveScaleX` -1.0))
  (:`Released`
    (goto _label)))

(event `Key|D`
  (params (Key :type "Key Structure"))
  ;[1 1 1] move left right keys
  (:`Pressed`
    (set `self.moveScaleY` 1.0))
  (:`Released`
    (goto _label_2)))

(fn `UserConstructionScript`)