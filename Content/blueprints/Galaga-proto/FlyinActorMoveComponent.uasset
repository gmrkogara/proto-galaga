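; FlyinActorMoveComponent is a movement component in a Galaga prototype that flies its owning actor toward MoveDestination.
; Every Tick calls UpdateLocation, which offsets the owner along the normalized direction to the destination, scaled by Velocity, without sweeping.
; DeltaSeconds is passed in but its multiply is left unconnected, so speed depends on frame rate, and no arrival check stops the movement.
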(event `self.ReceiveTick`
  (params (DeltaSeconds :type "Float (single-precision)"))
  (`self.update location` DeltaSeconds))

(event `update location`
  (params (`Delta seconds` :type "Float (double-precision)"))
  (`Actor.K2_AddActorWorldOffset` (`self.GetOwner`) (* (`KismetMathLibrary.Normal` (`KismetMathLibrary.GetDirectionUnitVector` (`Actor.K2_GetActorLocation` (`self.GetOwner`)) (`self.move destination`))) (`self.velocity`)) false false))