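; Temporary shield bubble actor that grants the Galaga player pawn an invincibility effect while it lasts.
; On spawn it caches the player's plane mesh and adds the effect, then moves its mesh to the plane's location every tick.
; Tick counts down the duration, plays a timeline driving transparency through a Material Parameter Collection in the final seconds, then destroys the bubble and removes the effect.
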(event `self.ReceiveBeginPlay`
  (`self.update location`)
  (bind _asgalaga_player_pawn (cast `/Game/blueprints/Galaga-proto/GalagaPlayerPawn` (`GameplayStatics.GetPlayerPawn` 0)))
  (set `self.Player plane mesh` (`/Game/blueprints/Galaga-proto/GalagaPlayerPawn.PlaneMesh` _asgalaga_player_pawn))
  (`/Game/blueprints/Galaga-proto/GalagaPlayerPawn.AddInvicibilityEffect` _asgalaga_player_pawn))

(event `self.ReceiveTick`
  (params (DeltaSeconds :type "Float (single-precision)"))
  (`self.update location`)
  (bind _output_get (set `self.Shiled duration` (- (`self.Shiled duration`) DeltaSeconds)))
  (if (< _output_get 0.0)
    (bind _asgalaga_player_pawn (cast `/Game/blueprints/Galaga-proto/GalagaPlayerPawn` (`GameplayStatics.GetPlayerPawn` 0)))
    (`self.K2_DestroyActor`)
    (`/Game/blueprints/Galaga-proto/GalagaPlayerPawn.RemoveInvicibilityEffect` _asgalaga_player_pawn)
    (elif (< (`self.Shiled duration`) 5.0)
      (`self.Animate`))))

(event `update location`
  (bind _player_plane_mesh (`self.Player plane mesh`))
  (if (`KismetSystemLibrary.IsValid` _player_plane_mesh)
    (`SceneComponent.K2_SetWorldLocation` (`self.StaticMeshComponent`) (`SceneComponent.K2_GetComponentLocation` _player_plane_mesh) false false)))

(event `Animate`
  (bind (_direction _transparency_output) (`Timeline|Timeline_0`)
    (:`Update`
      (`KismetMaterialLibrary.SetScalarParameterValue` "/Game/blueprints/Galaga-proto/ShieldBubblePMC.ShieldBubblePMC" "transparency" _transparency_output))))

(fn `UserConstructionScript`)