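; Player ship pawn for a Galaga-style shooter, handling banked impulse-driven side movement, firing, camera cycling, pause, score and HUD updates.
; A regenerating energy pool feeds shots and speed boost, with depletion briefly taking the reactor offline.
; Overlapped bonuses raise capped stats, add lives or spawn shields, with upgrade levels shown as ship meshes.
; Damage without invincibility costs a life, resets upgrades and combo, then spawns a shield or destroys the plane mesh.
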(event `update reactor energy`
  ;[1 1 1] update reactor energy
  (bind _output_get (set `self.Reactor online in` (`KismetMathLibrary.FClamp` (- (`self.Reactor online in`) (`self.delta seconds`)) 0.0 10.0)))
  (set `self.Is reactor working properly?` (not (> _output_get 0.0))))

(event `self.ReceiveAnyDamage`
  (params (Damage :type "Float (single-precision)") (DamageType :type "DamageType Object Reference") (InstigatedBy :type "Controller Object Reference") (DamageCauser :type "Actor Object Reference"))
  ;[1 1 1] any damage
  (`self.planeDestroyed`))

(event `self.ReceiveBeginPlay`
  (`self.GetHudWidget`)
  (bind _galaga_game_state (`/Game/blueprints/Galaga-proto/GalagaGlobalFunctions.Get galaga game state`))
  (set `self.galaga game state` _galaga_game_state))

(event `addToPlayerScore`
  (params (ScoreAmount :type Integer))
  (bind _hud_widget (`self.hud widget`))
  (bind _returnvalue (`KismetMathLibrary.FTrunc` (* ScoreAmount (`self.Score multiplier`))))
  ;[1 1 1] add score
  (set `self.Score` (+ (`self.Score`) _returnvalue))
  (`/Game/blueprints/Galaga-proto/GalagaGameHud.ShowJustScored` _hud_widget _returnvalue)
  (`/Game/blueprints/Galaga-proto/GalagaGameHud.AddValueToBonusBar` _hud_widget ScoreAmount))

(event `self.ReceiveTick`
  (params (DeltaSeconds :type "Float (single-precision)"))
  ;[1 1 1] event tick
  (bind _output_get (set `self.delta seconds` DeltaSeconds))
  (if (`KismetSystemLibrary.IsValid` (`self.PlaneMesh`))
    (`self.update reactor energy`)
    (`self.Reload ammo` _output_get)
    (`self.update collision box location`)
    (`self.update hud`)))

(event `self.bonus colission box.OnComponentBeginOverlap`
  (params (OverlappedComponent :type "PrimitiveComponent Object Reference") (OtherActor :type "Actor Object Reference") (OtherComp :type "PrimitiveComponent Object Reference") (OtherBodyIndex :type Integer) (bFromSweep :type Boolean) (SweepResult :type "HitResult Structure (by ref)"))
  ;[1 1 1] test if bonus overlaps player
  (if (== (`GameplayStatics.GetObjectClass` OtherActor) "/Game/blueprints/Galaga-proto/GalagaBonusBP.GalagaBonusBP_C")
    (bind _asgalaga_bonus_bp (cast `/Game/blueprints/Galaga-proto/GalagaBonusBP` OtherActor))
    (bind _bonustype (`/Game/blueprints/Galaga-proto/GalagaBonusBP.BonusType` _asgalaga_bonus_bp))
    (`self.Apply bonus to player` _bonustype)
    (if (or (== _bonustype (enumliteral `/Game/blueprints/Galaga-proto/BonusTypesEnum` "NewEnumerator5")) (== _bonustype (enumliteral `/Game/blueprints/Galaga-proto/BonusTypesEnum` "NewEnumerator6")))
      (`self.K2_DestroyActor` OtherActor)
      (else
        (`/Game/blueprints/Galaga-proto/GalagaBonusBP.start pick up animation` _asgalaga_bonus_bp)))))

(event `InputAxis|MoveRight`
  (params (AxisValue :type "Float (single-precision)"))
  (bind _planemesh (`self.PlaneMesh`))
  (bind _shiprotation (`self.ShipRotation`))
  ;[1 1 1] input handling
  ;;[1 1 1] play sides movement
  (if (`KismetSystemLibrary.IsValid` _planemesh)
    (`PrimitiveComponent.AddImpulse` _planemesh (`KismetMathLibrary.MakeVector` 0.0 (* (+ (`self.SideSpeed`) (`self.Static speed mod`)) AxisValue)) "None" true)
    (`|ExecutionSequence`
      (:`then_0`
        (if (== AxisValue 0.0)
          ;;[1 1 1] plane wing rotation
          (set `self.ShipRotation` (- _shiprotation (`KismetMathLibrary.SignOfFloat` _shiprotation)))
          (else
            (set `self.ShipRotation` (`KismetMathLibrary.FClamp` (+ _shiprotation AxisValue 0.0) -45.0 45.0))))
        (`SceneComponent.K2_SetWorldRotation` (`self.PlaneMesh`) (`KismetMathLibrary.MakeRotator` (`self.ShipRotation`)) false false))
      (:`then_1`
        ;;[1 1 1] energy consumption during speed mod on
        (if (and (!= AxisValue 0.0) (> (`self.Static speed mod`) 0.0))
          (set `self.ShipEnergy` (- (`self.ShipEnergy`) 0.02)))))))

(event `InputAction|Next camera`
  (params (Key :type "Key Structure"))
  ;[1 1 1] next camera
  (:`Pressed`
    (bind _output (`self.GetHudWidget`))
    (`|MultiGate` false true 1
      (:`Out 0`
        (`ActorComponent.SetActive` (`self.Camera1`) true false)
        (`ActorComponent.SetActive` (`self.Camera2`) false false)
        (`ActorComponent.SetActive` (`self.Camera3`) false false)
        (bind _targetbox (`/Game/blueprints/Galaga-proto/GalagaGameHud.targetBox` _output))
        (`Widget.SetVisibility` _targetbox "Collapsed"))
      (:`Out 1`
        (`ActorComponent.SetActive` (`self.Camera1`) false false)
        (`ActorComponent.SetActive` (`self.Camera2`) true false)
        (`ActorComponent.SetActive` (`self.Camera3`) false false))
      (:`Out 2`
        (`ActorComponent.SetActive` (`self.Camera1`) false false)
        (`ActorComponent.SetActive` (`self.Camera2`) false false)
        (`ActorComponent.SetActive` (`self.Camera3`) true false)
        (`Widget.SetVisibility` _targetbox "Visible")))))

(event `Reload ammo`
  (params (`delta seconds` :type "Float (double-precision)"))
  (bind _shipenergy (`self.ShipEnergy`))
  ;[1 1 1] reload ammo
  (if (< _shipenergy 0.0)
    (set `self.Reactor online in` 2.0))
  (if (< _shipenergy (`self.ShipEnergyMax`))
    (set `self.ShipEnergy` (`KismetMathLibrary.FClamp` (+ (`self.ShipEnergy`) (* (`self.Energy core regen rate`) `delta seconds`)) 0.0 (`self.ShipEnergyMax`)))))

(event `Apply bonus to player`
  (params (`Bonus type` :type "/Game/blueprints/Galaga-proto/BonusTypesEnum Enum" :default "NewEnumerator0"))
  ;[1 1 1] apply bonus to player
  (switch `/Game/blueprints/Galaga-proto/BonusTypesEnum` `Bonus type`
    (:`NewEnumerator0`
      (bind _returnvalue (`self.apply bonus to parameter` (`self.SideSpeed`) 30.0 3.0))
      (set `self.SideSpeed` _returnvalue)
      (`self.update bonus meshes` (`self.ShipSpeedBonusLvl`) (`self.shipSpeedBonuses`) "/Game/Meshes/EngineBonus_StaticMesh.EngineBonus_StaticMesh"))
    (:`NewEnumerator1`
      (bind _returnvalue_2 (`self.apply bonus to parameter` (`self.ShipEnergyMax`) 6.0 1.0))
      (set `self.ShipEnergyMax` _returnvalue_2)
      (`self.update bonus meshes` (`self.BulletAmmoBonusLvl`) (`self.bulletAmmoBonuses`) "/Game/Meshes/BulletAmmoBonus_StaticMesh.BulletAmmoBonus_StaticMesh"))
    (:`NewEnumerator3`
      (bind _returnvalue_3 (`self.apply bonus to parameter` (`self.Player bullet X Velocity`) 40.0 3.0))
      (set `self.Player bullet X Velocity` _returnvalue_3)
      (`self.update bonus meshes` (`self.BulletSpeedBonusLvl`) (`self.bulletSpeedBonuses`) "/Game/Meshes/BulletSpeedBonus_StaticMesh.BulletSpeedBonus_StaticMesh"))
    (:`NewEnumerator4`
      (`self.Cast new shield`))
    (:`NewEnumerator7`
      (bind _result (`/Engine/EditorBlueprintResources/StandardMacros.IncrementInt` (`self.Lives`))
        (:`  `
          (set `self.Lives` (`KismetMathLibrary.Clamp` _result 0 5)))))
    (:`NewEnumerator8`
      (bind _returnvalue_4 (`self.apply bonus to parameter` (`self.Energy core regen rate`) 2.0 0.3))
      (set `self.Energy core regen rate` _returnvalue_4))))

(event `update collision box location`
  ;[1 1 1] update plane collision box location
  (`SceneComponent.K2_SetWorldLocation` (`self.bonus colission box`) (.location (`SceneComponent.K2_GetComponentToWorld` (`self.PlaneMesh`))) false false))

(event `update hud`
  (bind _reactor_online_in (`self.Reactor online in`))
  ;[1 1 1] update hud
  (bind _output (`self.GetHudWidget`))
  (`|ExecutionSequence`
    (:`then_0`
      (`ProgressBar.SetPercent` (`/Game/blueprints/Galaga-proto/GalagaGameHud.pbBaseLife` _output) (/ (`KismetMathLibrary.Conv_IntToDouble` (`self.BaseLife`)) (`KismetMathLibrary.Conv_IntToDouble` (`self.BaseLifeMax`)))))
    (:`then_1`
      (`ProgressBar.SetPercent` (`/Game/blueprints/Galaga-proto/GalagaGameHud.pbShipEnergy` _output) (/ (`self.ShipEnergy`) (`self.ShipEnergyMax`))))
    (:`then_4`
      (`Widget.SetRenderOpacity` (`/Game/blueprints/Galaga-proto/GalagaGameHud.boxReactorOnlineIn` _output) _reactor_online_in)
      (`TextBlock.SetText` (`/Game/blueprints/Galaga-proto/GalagaGameHud.tbxReactorOnlineInSeconds` _output) (`KismetTextLibrary.Conv_DoubleToText` _reactor_online_in "HalfToEven" false true 1 324 0 1)))))

(event `InputAction|Fire weapon`
  (params (Key :type "Key Structure"))
  ;[1 1 1] spawn player bullet
  (:`Pressed`
    (if (`self.Is reactor working properly?`) :!label _label
      (`/Engine/EditorBlueprintResources/StandardMacros.IncrementInt` (`/Game/blueprints/Galaga-proto/GalagaGameState.ShootedBulletsCount` (`self.galaga game state`))
        (:`  `
          (`self.spawn player bullet` 50.0))))))

(event `Key|SpaceBar`
  (params (Key :type "Key Structure"))
  ;[1 1 1] spawn player bullet
  (:`Pressed`
    (goto _label)))

(event `Key|LeftMouseButton`
  (params (Key :type "Key Structure"))
  ;[1 1 1] spawn player bullet
  (:`Pressed`
    (goto _label)))

(event `InputAction|Speed modificator(shift)`
  (params (Key :type "Key Structure"))
  ;[1 1 1] speed mod input handling
  (:`Pressed`
    (if (and (> (`self.ShipEnergy`) 0.0) (`self.Is reactor working properly?`))
      (set `self.Static speed mod` (`self.Static speed modMax`))))
  (:`Released`
    (set `self.Static speed mod` 0.0)))

(event `InputAction|Pause Game`
  (params (Key :type "Key Structure"))
  (bind _returnvalue (`GameplayStatics.GetPlayerController` 0))
  ;[1 1 1] pause the game
  (:`Pressed`
    (`GameplayStatics.SetGamePaused` true)
    (bind _returnvalue_2 (`|CreateWidget` "/Game/blueprints/Galaga-proto/GalagaPauseMenu.GalagaPauseMenu_C" _returnvalue))
    (`UserWidget.AddToViewport` _returnvalue_2 0)
    (`WidgetBlueprintLibrary.SetInputMode_UIOnlyEx` _returnvalue _returnvalue_2)
    (set `PlayerController.bShowMouseCursor` true _returnvalue)))

(event `Key|B`
  (params (Key :type "Key Structure"))
  ;[1 1 1] force spawn bonus - for tests only
  (:`Pressed`
    (`|SpawnActorFromClass` "/Game/blueprints/Galaga-proto/GalagaBonusBP.GalagaBonusBP_C" (`KismetMathLibrary.MakeTransform` (`KismetMathLibrary.MakeVector` 1000.0 (`KismetMathLibrary.RandomFloatInRange` -1000.0 1000.0))) "Undefined" "OverrideRootScale" null null)))

(event `Cast new shield`
  ;[1 1 1] cast new shield
  (bind _outactors (`GameplayStatics.GetAllActorsOfClass` "/Game/blueprints/Galaga-proto/ShieldBubble_Blueprint.ShieldBubble_Blueprint_C"))
  (for _array_element _outactors
    (`self.RemoveInvicibilityEffect`)
    (`self.K2_DestroyActor` _array_element))
  (bind _returnvalue (`|SpawnActorFromClass` "/Game/blueprints/Galaga-proto/ShieldBubble_Blueprint.ShieldBubble_Blueprint_C" (`KismetMathLibrary.MakeTransform` (`SceneComponent.K2_GetComponentLocation` (`self.PlaneMesh`))) "Undefined" "OverrideRootScale" null null))
  (set `/Game/blueprints/Galaga-proto/ShieldBubble_Blueprint.Shiled duration` 30.0 _returnvalue)
  (bind _returnvalue_2 (`KismetMaterialLibrary.GetVectorParameterValue` "/Game/blueprints/Galaga-proto/BonusColorMaterialParameterCollection.BonusColorMaterialParameterCollection" "Cyan"))
  (`KismetMaterialLibrary.SetVectorParameterValue` "/Game/blueprints/Galaga-proto/ShieldBubblePMC.ShieldBubblePMC" "Color" _returnvalue_2))

(fn `AddInvicibilityEffect`
  (bind _result (`/Engine/EditorBlueprintResources/StandardMacros.IncrementInt` (`self.InvincibilityEffects`))
    (:`  `
      (set `self.InvincibilityEffects` _result))))

(fn `apply bonus to parameter`
  (params (`Current value` :type "Float (double-precision)") (`Max value` :type "Float (double-precision)") (`Value to add` :type "Float (double-precision)"))
  (returns (ReturnValue :type "Float (double-precision)"))
  (return (`KismetMathLibrary.FClamp` (+ `Current value` `Value to add`) 0.0 `Max value`)))

(fn `baseHit`
  (params (damage :type Integer))
  (set `self.BaseLife` (- (`self.BaseLife`) damage)))

(fn `clean bonus meshes`
  (for _array_element (`SceneComponent.GetChildrenComponents` (`self.bonuses`) true)
    (bind _asstatic_mesh_component (cast `StaticMeshComponent` _array_element))
    (`StaticMeshComponent.SetStaticMesh` _asstatic_mesh_component null))
  (return))

(fn `GetHudWidget`
  (returns (Output :type "/Game/blueprints/Galaga-proto/GalagaGameHud Object Reference"))
  (if (`KismetSystemLibrary.IsValid` (`self.hud widget`))
    (return (`self.hud widget`))
    (else
      (bind _foundwidgets (`WidgetBlueprintLibrary.GetAllWidgetsOfClass` "/Game/blueprints/Galaga-proto/GalagaGameHud.GalagaGameHud_C"))
      (bind _output_get (set `self.hud widget` (`|GetArrayItem` _foundwidgets)))
      (return _output_get))))

(fn `IsInvicible`
  (returns (IsInvincible :type Boolean))
  (return (> (`self.InvincibilityEffects`) 0)))

(fn `planeDestroyed`
  (if (`KismetSystemLibrary.IsValid` (`self.PlaneMesh`))
    (bind _isinvincible (`self.IsInvicible`))
    (if _isinvincible
      (`KismetSystemLibrary.PrintString` "Shield holding captain!")
      (else
        (bind _result (`/Engine/EditorBlueprintResources/StandardMacros.DecrementInt` (`self.Lives`))
          (:`  `
            (bind _asgalaga_game_mode (cast `/Game/blueprints/Galaga-proto/GalagaGameMode` (`GameplayStatics.GetGameMode`)))
            (`|ExecutionSequence`
              (:`then_0`
                (bind _output_get (set `self.Lives` _result)))
              (:`then_1`
                ;[1 1 1] clean bonus values and meshes
                (set `self.SideSpeed` (`/Game/blueprints/Galaga-proto/GalagaGameMode.Default side speed` _asgalaga_game_mode))
                (set `self.Player bullet X Velocity` (`/Game/blueprints/Galaga-proto/GalagaGameMode.Default player bullet X Velocity` _asgalaga_game_mode))
                (set `self.ShipEnergyMax` (`/Game/blueprints/Galaga-proto/GalagaGameMode.Default ammo count max` _asgalaga_game_mode))
                (set `self.BulletSpeedBonusLvl` 0)
                (set `self.ShipSpeedBonusLvl` 0)
                (set `self.BulletAmmoBonusLvl` 0))
              (:`then_2`
                (`self.clean bonus meshes`))
              (:`then_4`
                ;[1 1 1] cast shield bubble or remove plane from game
                (if (>= _output_get 0)
                  (`|SpawnActorFromClass` "/Game/blueprints/Galaga-proto/ShieldBubble_Blueprint.ShieldBubble_Blueprint_C" (`KismetMathLibrary.Conv_VectorToTransform` (`SceneComponent.K2_GetComponentLocation` (`self.PlaneMesh`))) "Undefined" "OverrideRootScale" null null)
                  (bind _returnvalue (`KismetMaterialLibrary.GetVectorParameterValue` "/Game/blueprints/Galaga-proto/BonusColorMaterialParameterCollection.BonusColorMaterialParameterCollection" "Red"))
                  (`KismetMaterialLibrary.SetVectorParameterValue` "/Game/blueprints/Galaga-proto/ShieldBubblePMC.ShieldBubblePMC" "Color" _returnvalue)
                  (else
                    (`ActorComponent.K2_DestroyComponent` (`self.PlaneMesh`)))))
              (:`then_5`
                ;[1 1 1] reset combo value
                (`/Game/blueprints/Galaga-proto/GalagaGameHud.AddValueToBonusBar` (`self.hud widget`) -9999)))))))))

(fn `RemoveInvicibilityEffect`
  (bind _result (`/Engine/EditorBlueprintResources/StandardMacros.DecrementInt` (`self.InvincibilityEffects`))
    (:`  `
      (set `self.InvincibilityEffects` _result))))

(fn `spawn player bullet`
  (params (LocationX :type "Float (double-precision)") (LocationY :type "Float (double-precision)"))
  (bind _planemesh (`self.PlaneMesh`))
  (bind _shipenergy (`self.ShipEnergy`))
  (bind _returnvalue (`SceneComponent.K2_GetComponentToWorld` _planemesh))
  (if (`KismetSystemLibrary.IsValid` _planemesh)
    (if (> _shipenergy 1.0)
      (bind _result (`/Engine/EditorBlueprintResources/StandardMacros.DecrementFloat` _shipenergy)
        (:`  `
          (set `self.ShipEnergy` _result)
          (bind _returnvalue_2 (`|SpawnActorFromClass` "/Game/blueprints/Galaga-proto/Enemy/EnemyBulletBp.EnemyBulletBp_C" (`KismetMathLibrary.MakeTransform` (`KismetMathLibrary.MakeVector` (+ (.x (.location _returnvalue)) LocationX) (+ (.y (.location _returnvalue)) LocationY))) "AlwaysSpawn" "OverrideRootScale" null false false 1 null))
          (bind _output_get (set `self.Bullet` _returnvalue_2))
          (`|ExecutionSequence`
            (:`then_0`
              (set `/Game/blueprints/Galaga-proto/Enemy/EnemyBulletBp.Velocity` (`KismetMathLibrary.MakeVector` (`self.Player bullet X Velocity`)) _output_get))
            (:`then_2`
              (set `/Game/blueprints/Galaga-proto/Enemy/EnemyBulletBp.IsArmed` true _output_get))
            (:`then_4`
              (bind _returnvalue_3 (`KismetMaterialLibrary.GetVectorParameterValue` "/Game/blueprints/Galaga-proto/BonusColorMaterialParameterCollection.BonusColorMaterialParameterCollection" "Yellow"))
              (`/Game/blueprints/Galaga-proto/Enemy/EnemyBulletBp.SetMaterialColor` _output_get _returnvalue_3)))))
      (else
        (set `self.Reactor online in` 2.0)))))

(fn `update bonus meshes`
  (params (`Bonus Lvl` :type "Integer (by ref)") (`Meshes container` :type "StaticMeshComponent Object Reference") (`bonus mesh` :type "StaticMesh Object Reference"))
  (`|ExecutionSequence`
    (:`then_0`
      (bind _asstatic_mesh_component (cast `StaticMeshComponent` (`|GetArrayItem` (`SceneComponent.GetChildrenComponents` `Meshes container` false) `Bonus Lvl`)))
      (`StaticMeshComponent.SetStaticMesh` _asstatic_mesh_component `bonus mesh`))
    (:`then_1`
      (bind _result (`/Engine/EditorBlueprintResources/StandardMacros.IncrementInt` `Bonus Lvl`)
        (:`  `
          (`|VariableSetRef` `Bonus Lvl` _result))))))

(fn `UserConstructionScript`
  (`|ExecutionSequence`
    (:`then_0`
      (`self.clean bonus meshes`)
      (for _array_element (`SceneComponent.GetChildrenComponents` (`self.bonuses`) true)
        (bind _asstatic_mesh_component (cast `StaticMeshComponent` _array_element))
        (`PrimitiveComponent.SetMaterial` _asstatic_mesh_component 0 "/Engine/BasicShapes/BasicShapeMaterial.BasicShapeMaterial")))
    (:`then_1`
      (for _array_element_2 (`SceneComponent.GetChildrenComponents` (`self.shipSpeedBonuses`) false)
        (bind _asstatic_mesh_component_2 (cast `StaticMeshComponent` _array_element_2))
        (`PrimitiveComponent.SetMaterial` _asstatic_mesh_component_2 0 "/Game/blueprints/mats/MatGreen.MatGreen")))
    (:`then_2`
      (for _array_element_3 (`SceneComponent.GetChildrenComponents` (`self.bulletSpeedBonuses`) false)
        (bind _asstatic_mesh_component_3 (cast `StaticMeshComponent` _array_element_3))
        (`PrimitiveComponent.SetMaterial` _asstatic_mesh_component_3 0 "/Game/blueprints/mats/MatYellow.MatYellow")))
    (:`then_3`
      (for _array_element_4 (`SceneComponent.GetChildrenComponents` (`self.bulletAmmoBonuses`) false)
        (bind _asstatic_mesh_component_4 (cast `StaticMeshComponent` _array_element_4))
        (`PrimitiveComponent.SetMaterial` _asstatic_mesh_component_4 0 "/Game/blueprints/mats/MatRed.MatRed")))))