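; Galaga bonus pickup actor that rolls a random bonus type on BeginPlay, coloring its mesh from a Material Parameter Collection and labeling it with camera-facing text.
; A timeline drives it along negative X with Y and Z motion.
; Reaching the player line applies base HP bonuses, clamped to max, with a pickup animation; other types are simply destroyed.
; Any damage destroys both it and the damage causer.
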(event `Bonus setup`
  (bind _staticmesh (`self.StaticMesh`))
  (bind _staticmesh_2 (`self.StaticMesh`))
  ;[1 1 1] setup bonus
  (`|ExecutionSequence`
    (:`then_0`
      (bind _output_get (set `self.BonusType` (cast `/Game/blueprints/Galaga-proto/BonusTypesEnum` (`KismetMathLibrary.Conv_IntToByte` (`KismetMathLibrary.RandomInteger` 7)))))
      (switch `/Game/blueprints/Galaga-proto/BonusTypesEnum` _output_get
        (:`NewEnumerator0`
          (bind _returnvalue (`KismetMaterialLibrary.GetVectorParameterValue` "/Game/blueprints/Galaga-proto/BonusColorMaterialParameterCollection.BonusColorMaterialParameterCollection" "Green"))
          (`/Game/blueprints/Galaga-proto/GalagaGlobalFunctions.Set mesh material color` (`self.StaticMesh`) _returnvalue))
        (:`NewEnumerator1`
          (bind _returnvalue_2 (`KismetMaterialLibrary.GetVectorParameterValue` "/Game/blueprints/Galaga-proto/BonusColorMaterialParameterCollection.BonusColorMaterialParameterCollection" "Blue"))
          (`/Game/blueprints/Galaga-proto/GalagaGlobalFunctions.Set mesh material color` _staticmesh_2 _returnvalue_2))
        (:`NewEnumerator3`
          (bind _returnvalue_3 (`KismetMaterialLibrary.GetVectorParameterValue` "/Game/blueprints/Galaga-proto/BonusColorMaterialParameterCollection.BonusColorMaterialParameterCollection" "Yellow"))
          (`/Game/blueprints/Galaga-proto/GalagaGlobalFunctions.Set mesh material color` _staticmesh_2 _returnvalue_3))
        (:`NewEnumerator4`
          (bind _returnvalue_4 (`KismetMaterialLibrary.GetVectorParameterValue` "/Game/blueprints/Galaga-proto/BonusColorMaterialParameterCollection.BonusColorMaterialParameterCollection" "Cyan"))
          (`/Game/blueprints/Galaga-proto/GalagaGlobalFunctions.Set mesh material color` _staticmesh_2 _returnvalue_4))
        (:`NewEnumerator5`
          (bind _returnvalue_5 (`KismetMaterialLibrary.GetVectorParameterValue` "/Game/blueprints/Galaga-proto/BonusColorMaterialParameterCollection.BonusColorMaterialParameterCollection" "Red"))
          (`/Game/blueprints/Galaga-proto/GalagaGlobalFunctions.Set mesh material color` _staticmesh _returnvalue_5))
        (:`NewEnumerator6`
          (bind _returnvalue_6 (`KismetMaterialLibrary.GetVectorParameterValue` "/Game/blueprints/Galaga-proto/BonusColorMaterialParameterCollection.BonusColorMaterialParameterCollection" "Magenta"))
          (`/Game/blueprints/Galaga-proto/GalagaGlobalFunctions.Set mesh material color` _staticmesh _returnvalue_6))
        (:`NewEnumerator7`
          (bind _returnvalue_7 (`KismetMaterialLibrary.GetVectorParameterValue` "/Game/blueprints/Galaga-proto/BonusColorMaterialParameterCollection.BonusColorMaterialParameterCollection" "Gray"))
          (`/Game/blueprints/Galaga-proto/GalagaGlobalFunctions.Set mesh material color` _staticmesh _returnvalue_7))))
    (:`then_2`
      (`TextRenderComponent.K2_SetText` (`self.TextRender`) (`KismetTextLibrary.Conv_StringToText` (`|GetEnumeratorNameAsString` (`self.BonusType`)))))))

(event `update text render to face camera`
  (bind (_returnvalue_roll _returnvalue_pitch _returnvalue_yaw) (`KismetMathLibrary.BreakRotator` (`SceneComponent.K2_GetComponentRotation` (`PlayerCameraManager.TransformComponent` (`PlayerController.PlayerCameraManager` (`GameplayStatics.GetPlayerController` 0))))))
  ;[1 1 1] update text render rotation to face the cam
  (`SceneComponent.K2_SetWorldRotation` (`self.TextRender`) (`KismetMathLibrary.MakeRotator` 0.0 (* _returnvalue_pitch -1.0) (+ _returnvalue_yaw 180.0)) false false))

(event `self.ReceiveAnyDamage`
  (params (Damage :type "Float (single-precision)") (DamageType :type "DamageType Object Reference") (InstigatedBy :type "Controller Object Reference") (DamageCauser :type "Actor Object Reference"))
  (`self.K2_DestroyActor` DamageCauser)
  (`self.K2_DestroyActor`))

(event `self.ReceiveTick`
  (params (DeltaSeconds :type "Float (single-precision)"))
  ;[1 1 1] event tick
  (`self.update text render to face camera`))

(event `self.ReceiveBeginPlay`
  ;[1 1 1] begin play
  (`|ExecutionSequence`
    (:`then_0`
      (`self.Bonus setup`))
    (:`then_1`
      (`self.start standard animation`))
    (:`then_2`
      (bind _asgalaga_player_pawn (cast `/Game/blueprints/Galaga-proto/GalagaPlayerPawn` (`GameplayStatics.GetPlayerPawn` 0)))
      (set `self.galaga player pawn` _asgalaga_player_pawn))))

(event `start standard animation`
  (bind _scene (`self.Scene`))
  (bind (_returnvalue_x _returnvalue_y) (`KismetMathLibrary.BreakVector` (`SceneComponent.K2_GetComponentLocation` _scene)))
  ;[1 1 1] move towards the players end animation
  (bind _output_get (set `self.initialYLocation` _returnvalue_y))
  (bind (_direction _float_0_1_0 _output_y) (`Timeline|Timeline_0-1-0` :!label _label)
    (:`Update`
      (`SceneComponent.K2_SetWorldLocation` _scene (`KismetMathLibrary.MakeVector` (+ _returnvalue_x -5.0) (+ _output_get (* _output_y 2.0)) _float_0_1_0) false false))))

(event `stop timeline animation`
  ;[1 1 1] move towards the players end animation
  (goto _label :!via `Stop`))

(event `self.ReceiveActorBeginOverlap`
  (params (OtherActor :type "Actor Object Reference"))
  (bind _bonustype (`self.BonusType`))
  (bind _baselifemax (`/Game/blueprints/Galaga-proto/GalagaPlayerPawn.BaseLifeMax` (`self.galaga player pawn`)))
  ;[1 1 1] overlap on player line collision box
  (bind _asgalaga_player_pawn (cast `/Game/blueprints/Galaga-proto/GalagaPlayerPawn` (`GameplayStatics.GetPlayerPawn` 0)))
  (bind _returnvalue (== (`/Game/blueprints/Galaga-proto/GalagaPlayerPawn.BulletBoxPlayerLine` _asgalaga_player_pawn) OtherActor))
  (if (and _returnvalue (or (`|EnumEquality` _bonustype "NewEnumerator5") (`|EnumEquality` _bonustype "NewEnumerator6")))
    (`|ExecutionSequence`
      (:`then_0`
        (switch `/Game/blueprints/Galaga-proto/BonusTypesEnum` (`self.BonusType`)
          (:`NewEnumerator5`
            (set `self.base life bonus` (/ _baselifemax 10)))
          (:`NewEnumerator6`
            (set `self.base life bonus` (/ _baselifemax 4)))))
      (:`then_1`
        (set `/Game/blueprints/Galaga-proto/GalagaPlayerPawn.BaseLife` (`KismetMathLibrary.Clamp` (+ (`/Game/blueprints/Galaga-proto/GalagaPlayerPawn.BaseLife` _asgalaga_player_pawn) (`self.base life bonus`)) 0 (`/Game/blueprints/Galaga-proto/GalagaPlayerPawn.BaseLifeMax` (`self.galaga player pawn`))) _asgalaga_player_pawn))
      (:`then_2`
        (`self.start pick up animation`)))
    (elif _returnvalue
      (`self.K2_DestroyActor`))))

(event `start pick up animation`
  (bind _scene (`self.Scene`))
  (bind (_relativelocation_x _relativelocation_y _relativelocation_z) (`KismetMathLibrary.BreakVector` (`SceneComponent.RelativeLocation` _scene)))
  ;[1 1 1] start pick up animation
  (`self.stop timeline animation`)
  (`ActorComponent.K2_DestroyComponent` (`self.StaticMesh`))
  (`KismetSystemLibrary.MoveComponentTo` _scene (`KismetMathLibrary.MakeVector` (+ _relativelocation_x 500.0) _relativelocation_y _relativelocation_z) (struct) false false 1.0)
  (`self.K2_DestroyActor`))

(fn `UserConstructionScript`)