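; Boss enemy for the Galaga prototype, built at BeginPlay from a random number of ShipPartBP child actors aligned in a centered row.
; It eases in from an offset via Timeline, then starts its parts shooting and randomly picks lateral destinations for FlyinActorMoveComponent.
; Hit points equal the part count and drop by one per damage event.
; At zero it destroys itself, signals BossIsDown and updates score and kill count.
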(event `self.ReceiveAnyDamage`
  (params (Damage :type "Float (single-precision)") (DamageType :type "DamageType Object Reference") (InstigatedBy :type "Controller Object Reference") (DamageCauser :type "Actor Object Reference"))
  (bind _ship_components (`self.ship components`))
  ;[1 1 1] any damage
  (`/Engine/EditorBlueprintResources/StandardMacros.DecrementInt` (`self.HitPoints`)
    (:`  `
      (`|ExecutionSequence`
        (:`then_0`
          (`KismetSystemLibrary.PrintString` "boss ship : component destroyed"))
        (:`then_1`
          (if (<= (`self.HitPoints`) 0)
            (`|ExecutionSequence`
              (:`then_0`
                (`KismetSystemLibrary.PrintString` "boss ship : destroyed"))
              (:`then_1`
                (for _array_element _ship_components
                  (`self.K2_DestroyActor` _array_element))
                (`KismetArrayLibrary.Array_Clear` _ship_components)
                (`self.Boss Is Down` (`self.Is Capital Ship`)))
              (:`then_2`
                (`/Game/blueprints/Galaga-proto/GalagaPlayerPawn.addToPlayerScore` (`self.galaga player pawn`) 10)
                (`self.K2_DestroyActor`))
              (:`then_3`
                (`/Engine/EditorBlueprintResources/StandardMacros.IncrementInt` (`/Game/blueprints/Galaga-proto/GalagaGameState.Enemies killed count` (`self.galaga game state`)))))))))))

(event `spawn component containers`
  ;[1 1 1] spawn ship components
  (for _ (range 1 (+ (`KismetMathLibrary.RandomIntegerInRange` (`self.Number of ship components min`) (`self.Number of ship components max`)) 1))
    (bind _returnvalue (`AddComponent|NODE_AddChildActorComponent-3`))
    (`ChildActorComponent.SetChildActorClass` _returnvalue "/Game/blueprints/Galaga-proto/Enemy/ShipPartBP.ShipPartBP_C")
    (bind _asship_part_bp (cast `/Game/blueprints/Galaga-proto/Enemy/ShipPartBP` (`ChildActorComponent.ChildActor` _returnvalue)))
    (bind _output_get (set `self.new ship component` _asship_part_bp))
    (`KismetArrayLibrary.Array_Add` (`self.ship components`) _output_get)
    (bind _staticmesh (`/Game/blueprints/Galaga-proto/Enemy/ShipPartBP.StaticMesh` _output_get))
    (`StaticMeshComponent.SetStaticMesh` _staticmesh "/Game/Meshes/blender/untitled_bulk.untitled_bulk")
    (`/Game/blueprints/Galaga-proto/GalagaGlobalFunctions.Set mesh material color` _staticmesh (`self.Color`))
    (set `self.HitPoints` (`KismetArrayLibrary.Array_Length` (`self.ship components`)))))

(event `self.ReceiveBeginPlay`
  ;[1 1 1] begin play
  (`|ExecutionSequence`
    (:`then_0`
      (set `/Game/blueprints/Galaga-proto/FlyinActorMoveComponent.move destination` (`self.K2_GetActorLocation`) (`self.FlyinActorMoveComponent`)))
    (:`then_1`
      (`self.spawn component containers`)
      (`self.align ship components`))
    (:`then_2`
      (bind _galaga_pawn (`/Game/blueprints/Galaga-proto/GalagaGlobalFunctions.Get galaga player pawn`))
      (set `self.galaga player pawn` _galaga_pawn)
      (bind _output (`/Game/blueprints/Galaga-proto/GalagaPlayerPawn.GetHudWidget` _galaga_pawn))
      (set `self.Hud widget` _output))
    (:`then_3`
      (bind _galaga_game_state (`/Game/blueprints/Galaga-proto/GalagaGlobalFunctions.Get galaga game state`))
      (set `self.galaga game state` _galaga_game_state))
    (:`then_4`
      (`self.slide in to battlefield`))))

(event `self.ReceiveTick`
  (params (DeltaSeconds :type "Float (single-precision)"))
  ;[1 1 1] event tick
  (if (`self.is ready to fight`)
    (if (<= (`KismetMathLibrary.RandomInteger` 1000) 3)
      (`self.create new move destination vector`))))

(event `align ship components`
  ;[1 1 1] align components to pivot center
  (for _array_element (`self.ship components`)
    (set `self.Ship width` (+ (`self.Ship width`) (* (.y (`.BoxExtent` (`self.GetActorBounds` _array_element false))) 2.0))))
  (for (_array_element_2 _array_index) (`self.ship components`)
    (bind (_origin _boxextent) (`self.GetActorBounds` _array_element_2 false))
    (bind _output_get (set `self.lastY` (.y _boxextent)))
    (`self.K2_SetActorRelativeLocation` _array_element_2 (`KismetMathLibrary.MakeVector` 0.0 (+ _output_get (+ (* _array_index (* (.y _boxextent) 2.0)) (* (/ (`self.Ship width`) 2.0) -1.0)))) false false)))

(event `create new move destination vector`
  (bind _returnvalue_x (`KismetMathLibrary.BreakVector` (`self.K2_GetActorLocation`)))
  (bind _returnvalue (- (`self.battlefield width`) (/ (`self.Ship width`) 2.0)))
  ;[1 1 1] create new move destination vector
  (bind _output_get (set `self.move destination` (`KismetMathLibrary.MakeVector` _returnvalue_x (`KismetMathLibrary.RandomFloatInRange` (* _returnvalue -1.0) _returnvalue))))
  (set `/Game/blueprints/Galaga-proto/FlyinActorMoveComponent.move destination` _output_get (`self.FlyinActorMoveComponent`)))

(event `slide in to battlefield`
  ;[1 1 1] slide in to battlefield
  (bind _output_get (set `self.slide in from` (`KismetMathLibrary.MakeVector` (`KismetMathLibrary.RandomFloatInRange` 400.0 600.0) (`KismetMathLibrary.RandomFloatInRange` -500.0 500.0) (`KismetMathLibrary.RandomFloatInRange` 1500.0 2000.0))))
  (bind _output_get_2 (set `self.position on lane` (`SceneComponent.K2_GetComponentLocation` (`self.DefaultSceneRoot`))))
  (bind (_direction _output_0_1) (`Timeline|Timeline_0`)
    (:`Update`
      (`SceneComponent.K2_SetWorldLocation` (`self.DefaultSceneRoot`) (`|EaseFunction` "EaseInOut" _output_0_1 (+ _output_get_2 _output_get) _output_get_2) false false))
    (:`Finished`
      (set `self.is ready to fight` true)
      (for _array_element (`self.GetAllChildActors` true)
        (bind _asship_part_bp (cast `/Game/blueprints/Galaga-proto/Enemy/ShipPartBP` _array_element))
        (`/Game/blueprints/Galaga-proto/Enemy/ShipPartBP.recalculate can shoot bullets` _asship_part_bp)
        (`/Game/blueprints/Galaga-proto/Enemy/ShipPartBP.start shooting bullets` _asship_part_bp)))))

(fn `UserConstructionScript`)