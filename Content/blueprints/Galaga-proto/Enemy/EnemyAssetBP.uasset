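; Base enemy Blueprint for a Galaga prototype that fires bullets at the player according to its enemy type.
; Attack spawns EnemyBulletBp in a delayed loop, with damage, speed and shot count selected by type.
; Bombers fire a ball-mesh bullet, Interceptors fire a burst aimed at the player's plane, and other types shoot straight along negative X.
; GetBulletStartingLocation returns zero here, and AreYouEnemy identifies the actor as an enemy.
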(event `Enemy Asset begin play`
  (bind _galaga_pawn (`/Game/blueprints/Galaga-proto/GalagaGlobalFunctions.Get galaga player pawn`))
  (set `self.Galaga player pawn` _galaga_pawn))

(event `self.ReceiveBeginPlay`
  (`self.Enemy Asset begin play`))

(event `/Game/blueprints/Galaga-proto/enemyPlaneAI/IBulletSpawner.Attack`
  (bind _returnvalue (`KismetMathLibrary.MakeRotator` 0.0))
  (bind _iterator (`self.iterator`))
  (bind (_bullet_starting_location_x _bullet_starting_location_y) (`KismetMathLibrary.BreakVector` (`self.bullet starting location`)))
  (bind _enemy_type (`self.Enemy Type`))
  (bind _returnvalue_2 (select `/Game/blueprints/Galaga-proto/Enemy/EnemyTypesEnum` _enemy_type :`NewEnumerator0` 20.0 :`NewEnumerator1` 20.0 :`NewEnumerator2` 30.0 :!type "Float (single-precision)"))
  ;[1 1 1] spawn bullet
  (bind _galaga_pawn (`/Game/blueprints/Galaga-proto/GalagaGlobalFunctions.Get galaga player pawn`))
  (set `self.Galaga player pawn` _galaga_pawn)
  (bind _vector (`self.get bullet starting location`))
  (set `self.bullet starting location` _vector)
  (set `self.iterator` 0)
  (`|ExecutionSequence` :!label _label
    (:`then_0`
      (bind _returnvalue_3 (`|SpawnActorFromClass` "/Game/blueprints/Galaga-proto/Enemy/EnemyBulletBp.EnemyBulletBp_C" (`KismetMathLibrary.MakeTransform` (`KismetMathLibrary.MakeVector` (+ _bullet_starting_location_x -150.0) _bullet_starting_location_y) (select `/Game/blueprints/Galaga-proto/Enemy/EnemyTypesEnum` (`self.Enemy Type`) :`NewEnumerator0` _returnvalue :`NewEnumerator1` _returnvalue :`NewEnumerator2` (`KismetMathLibrary.FindLookAtRotation` (`SceneComponent.K2_GetComponentLocation` (`self.DefaultSceneRoot`)) (`SceneComponent.K2_GetComponentLocation` (`/Game/blueprints/Galaga-proto/GalagaPlayerPawn.PlaneMesh` (`self.Galaga player pawn`)))))) "AlwaysSpawn" "OverrideRootScale" null (`self.Player Killer`) (`self.Is Armed`) (select `/Game/blueprints/Galaga-proto/Enemy/EnemyTypesEnum` (`self.Enemy Type`) :`NewEnumerator0` 1 :`NewEnumerator1` 3) null))
      (if (== (`self.Enemy Type`) (enumliteral `/Game/blueprints/Galaga-proto/Enemy/EnemyTypesEnum` "NewEnumerator1"))
        (bind _bullet_mesh (`/Game/blueprints/Galaga-proto/Enemy/EnemyBulletBp.bullet mesh` _returnvalue_3))
        (`StaticMeshComponent.SetStaticMesh` _bullet_mesh "/Game/Meshes/Ball_StaticMesh.Ball_StaticMesh")
        (`SceneComponent.SetWorldScale3D` _bullet_mesh (1.0 1.0 1.0)))
      (bind _output_get (set `self.Bullet` _returnvalue_3))
      (if (`KismetSystemLibrary.IsValid` _output_get)
        (`|ExecutionSequence`
          (:`then_3`
            (`/Game/blueprints/Galaga-proto/Enemy/EnemyBulletBp.SetMaterialColor` _output_get (struct :`R` 1.0 :`G` 1.0 :`B` 1.0 :`A` 1.0)))
          (:`then_4`
            (if (not (== _enemy_type (enumliteral `/Game/blueprints/Galaga-proto/Enemy/EnemyTypesEnum` "NewEnumerator2")))
              (set `/Game/blueprints/Galaga-proto/Enemy/EnemyBulletBp.Velocity` (`KismetMathLibrary.MakeVector` (* _returnvalue_2 -1.0)) _output_get)
              (else
                (set `/Game/blueprints/Galaga-proto/Enemy/EnemyBulletBp.Velocity` (* (`KismetMathLibrary.Normal` (`KismetMathLibrary.GetDirectionUnitVector` (`SceneComponent.K2_GetComponentLocation` (`self.DefaultSceneRoot`)) (`SceneComponent.K2_GetComponentLocation` (`/Game/blueprints/Galaga-proto/GalagaPlayerPawn.PlaneMesh` (`self.Galaga player pawn`))))) _returnvalue_2) _output_get)))))))
    (:`then_1`
      (`/Engine/EditorBlueprintResources/StandardMacros.IncrementInt` _iterator))
    (:`then_2`
      (if (< _iterator (select `/Game/blueprints/Galaga-proto/Enemy/EnemyTypesEnum` (`self.Enemy Type`) :`NewEnumerator0` 1 :`NewEnumerator1` 1 :`NewEnumerator2` 3))
        (`KismetSystemLibrary.Delay` 0.3)
        (goto _label)))))

(fn `Are you enemy`
  (returns (`are you ?` :type Boolean))
  (return true))

(fn `get bullet starting location`
  (returns (Vector :type "Vector Structure"))
  (return (0.0 0.0 0.0)))

(fn `UserConstructionScript`
  (bind _galaga_pawn (`/Game/blueprints/Galaga-proto/GalagaGlobalFunctions.Get galaga player pawn`))
  (set `self.Galaga player pawn` _galaga_pawn))