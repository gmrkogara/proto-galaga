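; Enemy plane pawn for the Galaga prototype, configured by EnemyType as Aircraft, Bomber or Interceptor.
; BeginPlay sets the matching child-actor plane and color, caches the player and spawns its AI controller; setup eases it into its lane from a random offset.
; spawnbullet fires per type: straight shots, ball-mesh bombs, or delayed bursts aimed at the player.
; Any damage destroys it and the damage causer, awards score and may drop a bonus.
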(event `self.ReceiveBeginPlay`
  (bind _enemyplaneactor (`self.EnemyPlaneActor`))
  (`|ExecutionSequence`
    (:`then_0`
      (bind _asactor (castclass `Actor` (select `/Game/blueprints/Galaga-proto/Enemy/EnemyTypesEnum` (`self.Enemy Type`) :`NewEnumerator0` "/Game/Meshes/blender/airplaneBP.airplaneBP_C" :`NewEnumerator1` "/Game/Meshes/blender/bomberBP.bomberBP_C" :`NewEnumerator2` "/Game/Meshes/blender/interceptorBP.interceptorBP_C" :!type "Object Class Reference")))
      (`ChildActorComponent.SetChildActorClass` _enemyplaneactor _asactor)
      (bind _asbase_airplane_bp (cast `/Game/Meshes/blender/baseAirplaneBP` (`ChildActorComponent.ChildActor` _enemyplaneactor)))
      (`/Game/Meshes/blender/baseAirplaneBP.set plane material color` _asbase_airplane_bp (select `/Game/blueprints/Galaga-proto/Enemy/EnemyTypesEnum` (`self.Enemy Type`) :`NewEnumerator0` (`KismetMathLibrary.LinearColor_Green`) :`NewEnumerator1` (`KismetMathLibrary.LinearColor_Red`) :`NewEnumerator2` (`KismetMathLibrary.LinearColor_Yellow`))))
    (:`then_1`
      (bind _asgalaga_player_pawn (cast `/Game/blueprints/Galaga-proto/GalagaPlayerPawn` (`GameplayStatics.GetPlayerPawn` 0)))
      (set `self.Galaga player pawn` _asgalaga_player_pawn))
    (:`then_3`
      (set `self.AIControllerClass` "/Game/blueprints/Galaga-proto/enemyPlaneAI/EnemyPlaneController.EnemyPlaneController_C")
      (`self.SpawnDefaultController`))))

(event `self.ReceiveAnyDamage`
  (params (Damage :type "Float (single-precision)") (DamageType :type "DamageType Object Reference") (InstigatedBy :type "Controller Object Reference") (DamageCauser :type "Actor Object Reference"))
  ;[1 1 1] any damage event
  (`|ExecutionSequence`
    (:`then_0`
      (if (< (`KismetMathLibrary.RandomFloatInRange` 0.0 100.0) 10.0)
        (`|SpawnActorFromClass` "/Game/blueprints/Galaga-proto/GalagaBonusBP.GalagaBonusBP_C" (`KismetMathLibrary.MakeTransform` (`SceneComponent.K2_GetComponentLocation` (`self.Scene`))) "Undefined" "OverrideRootScale" null null)))
    (:`then_1`
      (`self.K2_DestroyActor` DamageCauser))
    (:`then_2`
      (`/Game/blueprints/Galaga-proto/GalagaPlayerPawn.addToPlayerScore` (`self.Galaga player pawn`) (select `/Game/blueprints/Galaga-proto/Enemy/EnemyTypesEnum` (`self.Enemy Type`) :`NewEnumerator0` 3 :`NewEnumerator1` 6 :`NewEnumerator2` 9))
      (`self.K2_DestroyActor`))))

(event `setup`
  (bind _output_get (set `self.slide in from` (`KismetMathLibrary.MakeVector` (`KismetMathLibrary.RandomFloatInRange` 400.0 600.0) (`KismetMathLibrary.RandomFloatInRange` -500.0 500.0) (`KismetMathLibrary.RandomFloatInRange` 1500.0 2000.0))))
  (bind _output_get_2 (set `self.position on lane` (`SceneComponent.K2_GetComponentLocation` (`self.Scene`))))
  (bind (_direction _output_0_1) (`Timeline|Timeline_0`)
    (:`Update`
      (`SceneComponent.K2_SetWorldLocation` (`self.Scene`) (`|EaseFunction` "EaseInOut" _output_0_1 (+ _output_get_2 _output_get) _output_get_2) false false))))

(event `spawn bullet`
  (bind _returnvalue (`KismetMathLibrary.MakeRotator` 0.0))
  (bind _iterator (`self.iterator`))
  (bind _enemy_type (`self.Enemy Type`))
  (bind _returnvalue_2 (`SceneComponent.K2_GetComponentToWorld` (`self.EnemyPlaneActor`)))
  (bind _returnvalue_3 (select `/Game/blueprints/Galaga-proto/Enemy/EnemyTypesEnum` _enemy_type :`NewEnumerator0` 20.0 :`NewEnumerator1` 20.0 :`NewEnumerator2` 30.0 :!type "Float (single-precision)"))
  ;[1 1 1] spawn bullet
  (set `self.iterator` 0)
  (`|ExecutionSequence` :!label _label
    (:`then_0`
      (bind _returnvalue_4 (`|SpawnActorFromClass` "/Game/blueprints/Galaga-proto/Enemy/EnemyBulletBp.EnemyBulletBp_C" (`KismetMathLibrary.MakeTransform` (`KismetMathLibrary.MakeVector` (+ (.x (.location _returnvalue_2)) -150.0) (.y (.location _returnvalue_2))) (select `/Game/blueprints/Galaga-proto/Enemy/EnemyTypesEnum` (`self.Enemy Type`) :`NewEnumerator0` _returnvalue :`NewEnumerator1` _returnvalue :`NewEnumerator2` (`KismetMathLibrary.FindLookAtRotation` (`SceneComponent.K2_GetComponentLocation` (`self.Scene`)) (`SceneComponent.K2_GetComponentLocation` (`/Game/blueprints/Galaga-proto/GalagaPlayerPawn.PlaneMesh` (`self.Galaga player pawn`)))))) "AlwaysSpawn" "OverrideRootScale" null false false (select `/Game/blueprints/Galaga-proto/Enemy/EnemyTypesEnum` (`self.Enemy Type`) :`NewEnumerator0` 1 :`NewEnumerator1` 3) null))
      (if (== (`self.Enemy Type`) (enumliteral `/Game/blueprints/Galaga-proto/Enemy/EnemyTypesEnum` "NewEnumerator1"))
        (bind _bullet_mesh (`/Game/blueprints/Galaga-proto/Enemy/EnemyBulletBp.bullet mesh` _returnvalue_4))
        (`StaticMeshComponent.SetStaticMesh` _bullet_mesh "/Game/Meshes/Ball_StaticMesh.Ball_StaticMesh")
        (`SceneComponent.SetWorldScale3D` _bullet_mesh (1.0 1.0 1.0)))
      (bind _output_get (set `self.Bullet` _returnvalue_4))
      (if (`KismetSystemLibrary.IsValid` _output_get)
        (`|ExecutionSequence`
          (:`then_0`
            (set `/Game/blueprints/Galaga-proto/Enemy/EnemyBulletBp.PlayerKiller` true _output_get))
          (:`then_2`
            (set `/Game/blueprints/Galaga-proto/Enemy/EnemyBulletBp.IsArmed` true _output_get))
          (:`then_3`
            (`/Game/blueprints/Galaga-proto/Enemy/EnemyBulletBp.SetMaterialColor` _output_get (struct :`R` 1.0 :`G` 1.0 :`B` 1.0 :`A` 1.0)))
          (:`then_4`
            (if (not (== _enemy_type (enumliteral `/Game/blueprints/Galaga-proto/Enemy/EnemyTypesEnum` "NewEnumerator2")))
              (set `/Game/blueprints/Galaga-proto/Enemy/EnemyBulletBp.Velocity` (`KismetMathLibrary.MakeVector` (* _returnvalue_3 -1.0)) _output_get)
              (else
                (set `/Game/blueprints/Galaga-proto/Enemy/EnemyBulletBp.Velocity` (* (`KismetMathLibrary.Normal` (`KismetMathLibrary.GetDirectionUnitVector` (`SceneComponent.K2_GetComponentLocation` (`self.Scene`)) (`SceneComponent.K2_GetComponentLocation` (`/Game/blueprints/Galaga-proto/GalagaPlayerPawn.PlaneMesh` (`self.Galaga player pawn`))))) _returnvalue_3) _output_get)))))))
    (:`then_1`
      (`/Engine/EditorBlueprintResources/StandardMacros.IncrementInt` _iterator))
    (:`then_2`
      (if (< _iterator (select `/Game/blueprints/Galaga-proto/Enemy/EnemyTypesEnum` (`self.Enemy Type`) :`NewEnumerator0` 1 :`NewEnumerator1` 1 :`NewEnumerator2` 3))
        (`KismetSystemLibrary.Delay` 0.3)
        (goto _label)))))

(fn `UserConstructionScript`)