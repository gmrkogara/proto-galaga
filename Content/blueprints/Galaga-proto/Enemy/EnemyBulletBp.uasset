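; Galaga projectile whose PlayerKiller flag sets whether it hurts the player or enemies.
; It moves by Velocity each Tick and, when armed, resolves overlaps: boundary boxes count a miss or damage the base, while valid targets get a boom and damage.
; When damaged itself, it may spawn a bonus scaled by score multiplier, destroys the damage causer, awards score and destroys itself.
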(event `self.ReceiveBeginPlay`
  (bind _asgalaga_player_pawn (cast `/Game/blueprints/Galaga-proto/GalagaPlayerPawn` (`GameplayStatics.GetPlayerPawn` 0)))
  (set `self.GalagaPlayerPawn` _asgalaga_player_pawn)
  (bind _galaga_game_state (`/Game/blueprints/Galaga-proto/GalagaGlobalFunctions.Get galaga game state`))
  (set `self.galaga game state` _galaga_game_state))

(event `self.ReceiveTick`
  (params (DeltaSeconds :type "Float (single-precision)"))
  (`self.update location`))

(event `update location`
  ;[1 1 1] update location
  (`SceneComponent.K2_AddRelativeLocation` (`self.Scene`) (`self.Velocity`) false false))

(event `self.bullet mesh.OnComponentBeginOverlap`
  (params (OverlappedComponent :type "PrimitiveComponent Object Reference") (OtherActor :type "Actor Object Reference") (OtherComp :type "PrimitiveComponent Object Reference") (OtherBodyIndex :type Integer) (bFromSweep :type Boolean) (SweepResult :type "HitResult Structure (by ref)"))
  (bind _galagaplayerpawn (`self.GalagaPlayerPawn`))
  ;[1 1 1] kills on overlap
  (`|ExecutionSequence`
    (:`then_0`
      (if (`self.IsArmed`)
        (if (== OtherActor (`/Game/blueprints/Galaga-proto/GalagaPlayerPawn.BulletBoxEnemyLine` _galagaplayerpawn))
          (`/Engine/EditorBlueprintResources/StandardMacros.IncrementInt` (`/Game/blueprints/Galaga-proto/GalagaGameState.MissedBulletsCount` (`self.galaga game state`))
            (:`  `
              (`self.K2_DestroyActor` :!label _label)))
          (elif (== OtherActor (`/Game/blueprints/Galaga-proto/GalagaPlayerPawn.BulletBoxPlayerLine` _galagaplayerpawn))
            (`/Game/blueprints/Galaga-proto/GalagaPlayerPawn.baseHit` (`self.GalagaPlayerPawn`) (`self.BaseHpDamage`))
            (goto _label)
            (elif (and (`self.PlayerKiller`) (== "/Game/blueprints/Galaga-proto/GalagaPlayerPawn.GalagaPlayerPawn_C" (`GameplayStatics.GetObjectClass` OtherActor)))
              (`self.show boom` (0.0 0.0 0.0) :!label _label_2)
              (`GameplayStatics.ApplyDamage` OtherActor 1.0 null self)
              (else
                (bind _are_you__ (message `/Game/blueprints/Galaga-proto/Enemy/IEnemyAsset.Are you enemy` OtherActor))
                (if (and _are_you__ (not (`self.PlayerKiller`)))
                  (goto _label_2))))))))))

(event `self.ReceiveAnyDamage`
  (params (Damage :type "Float (single-precision)") (DamageType :type "DamageType Object Reference") (InstigatedBy :type "Controller Object Reference") (DamageCauser :type "Actor Object Reference"))
  ;[1 1 1] any damage
  (`KismetSystemLibrary.PrintString` "bullet any damage")
  (`|ExecutionSequence`
    (:`then_0`
      (if (< (`KismetMathLibrary.RandomFloatInRange` 0.0 100.0) (* (`/Game/blueprints/Galaga-proto/GalagaPlayerPawn.Score multiplier` (`self.GalagaPlayerPawn`)) (`self.bonus spawn chance`)))
        (bind _returnvalue (`|SpawnActorFromClass` "/Game/blueprints/Galaga-proto/GalagaBonusBP.GalagaBonusBP_C" (`KismetMathLibrary.MakeTransform` (`SceneComponent.K2_GetComponentLocation` (`self.bullet mesh`))) "Undefined" "OverrideRootScale" null null))
        (`KismetSystemLibrary.PrintString` (`KismetSystemLibrary.GetDisplayName` _returnvalue))))
    (:`then_1`
      (`/Engine/EditorBlueprintResources/StandardMacros.IsValid` DamageCauser
        (:`Is Valid`
          (`self.K2_DestroyActor` DamageCauser))))
    (:`then_2`
      (`/Game/blueprints/Galaga-proto/GalagaPlayerPawn.addToPlayerScore` (`self.GalagaPlayerPawn`) 5)
      (`/Engine/EditorBlueprintResources/StandardMacros.IsValid` self
        (:`Is Valid`
          (`self.K2_DestroyActor`))))))

(event `update score`
  (params (socre :type Integer))
  ;[1 1 1] update score
  (`/Game/blueprints/Galaga-proto/GalagaPlayerPawn.addToPlayerScore` (`self.GalagaPlayerPawn`) socre))

(event `spawn bonus`
  (params (chance :type "Float (double-precision)") (location :type "Vector Structure"))
  ;[1 1 1] spawn bonus
  (`|ExecutionSequence`
    (:`then_0`
      (if (< (`KismetMathLibrary.RandomFloatInRange` 0.0 100.0) chance)
        (`|SpawnActorFromClass` "/Game/blueprints/Galaga-proto/GalagaBonusBP.GalagaBonusBP_C" (`KismetMathLibrary.MakeTransform` location) "Undefined" "OverrideRootScale" null null)))))

(event `on enemy entity hit`
  (params (`enemy entity` :type "Actor Object Reference") (`spawn change` :type "Float (double-precision)") (score :type Integer))
  ;[1 1 1] on enemy entity hit
  (`self.K2_DestroyActor` `enemy entity`)
  (`self.update score` score)
  (`self.spawn bonus` `spawn change` (`SceneComponent.K2_GetComponentLocation` (`self.Scene`))))

(event `show boom`
  (params (Location :type "Vector Structure"))
  ;[1 1 1] show boom
  (`|ExecutionSequence`
    (:`then_0`
      (`|SpawnActorFromClass` "/Game/blueprints/Galaga-proto/GalagaboomBP.GalagaBoomBP_C" (`KismetMathLibrary.MakeTransform` (`SceneComponent.K2_GetComponentLocation` (`self.Scene`))) "Undefined" "OverrideRootScale" null null))))

(fn `Are you enemy`
  (returns (`are you ?` :type Boolean))
  (return (`self.PlayerKiller`)))

(fn `SetMaterialColor`
  (params (`Linear Color` :type "LinearColor Structure"))
  (`/Game/blueprints/Galaga-proto/GalagaGlobalFunctions.Set mesh material color` (`self.bullet mesh`) `Linear Color`))

(fn `UserConstructionScript`)