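; Enemy spawner for the Galaga prototype that drives waves, bosses and stage progression.
; A random-delay loop spawns small ships into free lanes or announced minibosses, scaled by stage and game tier.
; A growing spawn-count threshold clears the field for a level boss, whose defeat advances the stage and shortens delays.
; Bosses share one parameterized spawn event reporting death through a delegate; E and R keys also trigger spawns.
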(event `self.ReceiveBeginPlay`
  (set `self.Spawn boss at` 3)
  (`self.spawn enemy`))

(event `Key|R`
  (params (Key :type "Key Structure"))
  (:`Pressed`
    (`self.spawn boss ship` 2 5)))

(event `show annoucement`
  (params (Duration :type "Float (double-precision)") (Text :type Text))
  ;[1 1 1] show info boss incomming
  (bind _galaga_pawn (`/Game/blueprints/Galaga-proto/GalagaGlobalFunctions.Get galaga player pawn`))
  (bind _output (`/Game/blueprints/Galaga-proto/GalagaPlayerPawn.GetHudWidget` _galaga_pawn))
  (`/Game/blueprints/Galaga-proto/GalagaGameHud.Show announcement bar` _output Text Duration))

(event `Spawn corvette ship boss`
  (params (color :type "LinearColor Structure" :default (struct :`G` 1.0 :`B` 0.090284 :`A` 1.0)))
  ;[1 1 1] spawn boss events
  (`self.spawn boss ship` 1 3 false color))

(event `spawn mini boss`
  ;[1 1 1] spawn boss events
  (if (<= (`KismetMathLibrary.RandomIntegerInRange` 1 15) (`self.current stage`))
    (`self.Spawn capital ship boss` false (struct :`R` 0.755208 :`G` 0.534274 :`A` 1.0))
    (else
      (`self.Spawn corvette ship boss` (struct :`G` 1.0 :`B` 0.090284 :`A` 1.0)))))

(event `Key|E`
  (params (Key :type "Key Structure"))
  ;[1 1 1] spawn random enemy
  (:`Pressed`
    (if (< (`KismetMathLibrary.RandomInteger` 100) (`self.Cance to spawn random boss`)) :!label _label
      (bind _game_tier (`/Game/blueprints/Galaga-proto/GalagaGlobalFunctions.Get game tier` true))
      (if (< (`self.number of boss ships`) _game_tier)
        (`self.show annoucement` 2.0 "Unknown ship incomming")
        (`KismetSystemLibrary.Delay` 3.0)
        (`self.spawn mini boss`)
        (else
          (if (== (`self.number of boss ships`) 0) :!label _label_2
            (for _ (range (+ (`KismetMathLibrary.RandomInteger` (`.ReturnValue` (`KismetMathLibrary.FMod` (`KismetMathLibrary.Conv_IntToDouble` (`self.current stage`)) 4.0))) 1))
              (`self.spawn small ship`)
              (`KismetSystemLibrary.Delay` 0.2))
            (else
              (`KismetSystemLibrary.Delay` 5.0)))))
      (else
        (goto _label_2)))
    (`self.spawn enemy`)))

(event `Spawn capital ship boss`
  (params (`is end level boss` :type Boolean) (Color :type "LinearColor Structure" :default (struct :`R` 0.973687 :`G` 1.0 :`A` 1.0)))
  ;[1 1 1] spawn boss events
  (`self.spawn boss ship` 2 4 `is end level boss` Color))

(event `spawn enemy`
  ;[1 1 1] spawn random enemy
  (`KismetSystemLibrary.Delay` (`KismetMathLibrary.RandomFloatInRange` (`self.Min Duration betwen spawns`) (`self.Max Duration betwen spawns`)))
  (goto _label))

(event `spawn level boss`
  ;[1 1 1] spawn boss events
  (if (<= (`KismetMathLibrary.RandomIntegerInRange` 1 15) (`self.current stage`))
    (`self.Spawn mega ship boss` true)
    (else
      (`self.Spawn capital ship boss` true))))

(event `Spawn mega ship boss`
  (params (`is end level boss` :type Boolean) (Color :type "LinearColor Structure" :default (struct :`R` 1.0 :`G` 0.096654 :`A` 1.0)))
  ;[1 1 1] spawn boss events
  (`self.spawn boss ship` 3 7 `is end level boss` Color))

(event `spawn small ship`
  (bind _returnvalue (`SceneComponent.K2_GetComponentToWorld` (`self.DefaultSceneRoot`)))
  ;[1 1 1] spawn small ship
  (bind _outactors (`GameplayStatics.GetAllActorsOfClass` "/Game/blueprints/Galaga-proto/Enemy/EnemyPlaneBP.EnemyPlaneBP_C"))
  (if (< (`KismetArrayLibrary.Array_Length` _outactors) 20)
    (bind _lane (`self.GetEnemyLane`))
    (set `self.lane` _lane)
    (bind (_returnvalue_2 _hitpoints _tier) (`self.Get new ship type`))
    (`|SpawnActorFromClass` "/Game/blueprints/Galaga-proto/Enemy/EnemyPlaneBP_2.EnemyPlaneBP_2_C" (`KismetMathLibrary.MakeTransform` (`KismetMathLibrary.MakeVector` (.x (.location _returnvalue)) (+ (* _lane 200.0) 100.0) (.z (.location _returnvalue))) (struct :`Yaw` 180.0)) "Undefined" "OverrideRootScale" null (`self.lane`) _hitpoints _tier _returnvalue_2 null)
    (`|ExecutionSequence`
      (:`then_0`
        (bind _result (`/Engine/EditorBlueprintResources/StandardMacros.IncrementInt` (`self.Spawned enemies count`))
          (:`  `
            (if (== _result (`self.Spawn boss at`))
              (`|ExecutionSequence`
                (:`then_0`
                  (`self.show annoucement` 3.0 "Capital Ship Incomming")
                  (`KismetSystemLibrary.Delay` 5.0)
                  (`self.despawn small ships`)
                  (`self.despawn mini bosses`)
                  (`self.spawn level boss`))
                (:`then_1`
                  (set `self.Spawn boss at` (+ (`KismetMathLibrary.FTrunc` (* (`self.Spawn boss at`) 1.4)) (`self.Spawn boss at`))))))))))
    (else
      (`KismetSystemLibrary.PrintString` "20 enemies is enough")
      (`KismetSystemLibrary.Delay` 10.0)
      (`self.spawn small ship`))))

(event `spawn boss ship`
  (params (`min number of components` :type Integer) (`max number of components` :type Integer) (`is capital ship` :type Boolean) (Color :type "LinearColor Structure" :default (struct :`R` 0.890625 :`G` 0.890625 :`B` 0.890625 :`A` 1.0)))
  ;[1 1 1] spawn boss ship
  (`/Engine/EditorBlueprintResources/StandardMacros.IncrementInt` (`self.number of boss ships`)
    (:`  `
      (bind _returnvalue (`|SpawnActorFromClass` "/Game/blueprints/Galaga-proto/Enemy/EnemyBossBP.EnemyBossBP_C" (`KismetMathLibrary.MakeTransform` (`KismetMathLibrary.MakeVector` (`KismetMathLibrary.RandomFloatInRange` 3500.0 4000.0) (`KismetMathLibrary.RandomFloatInRange` -1000.0 1000.0))) "Undefined" "OverrideRootScale" null `min number of components` `max number of components` `is capital ship` Color null))
      (add `/Game/blueprints/Galaga-proto/Enemy/EnemyBossBP.Boss Is Down` _returnvalue (delegate `On Boss Is Down`)))))

(event `On Boss Is Down`
  (params (`is capital ship` :type Boolean))
  ;[1 1 1] spawn boss ship
  (`/Engine/EditorBlueprintResources/StandardMacros.DecrementInt` (`self.number of boss ships`)
    (:`  `
      (if `is capital ship`
        (bind _string (`self.format stage completed text`))
        (bind _output_get (set `self.stage completed text` _string))
        (`self.show annoucement` 3.0 (`KismetTextLibrary.Conv_StringToText` _output_get))
        (bind _result (`/Engine/EditorBlueprintResources/StandardMacros.IncrementInt` (`self.current stage`))
          (:`  `
            (bind _asgalaga_game_state (cast `/Game/blueprints/Galaga-proto/GalagaGameState` (`GameplayStatics.GetGameState`)))
            (set `/Game/blueprints/Galaga-proto/GalagaGameState.Game Stage` _result _asgalaga_game_state)
            (`self.reduce spawn delays`))))
      (set `self.Cance to spawn random boss` (`KismetMathLibrary.Clamp` (+ (`self.Cance to spawn random boss`) 2) 0 20))
      (`self.spawn enemy`))))

(event `despawn small ships`
  ;[1 1 1] despawn ships/booses
  (bind _outactors (`GameplayStatics.GetAllActorsOfClass` "/Game/blueprints/Galaga-proto/Enemy/EnemyPlaneBP_2.EnemyPlaneBP_2_C"))
  (bind _output_get (set `self.ship for despawn` _outactors))
  (for _index (range (+ (`KismetMathLibrary.FTrunc` (* (`KismetArrayLibrary.Array_Length` _outactors) 0.9)) 1))
    (`/Game/blueprints/Galaga-proto/Enemy/EnemyPlaneBP_2.move out of field` (`|GetArrayItem` _output_get _index))
    (`KismetSystemLibrary.Delay` 0.2)))

(event `reduce spawn delays`
  ;[1 1 1] reduce spawn delays
  (set `self.Max Duration betwen spawns` (`KismetMathLibrary.FClamp` (* 0.98 (`self.Max Duration betwen spawns`)) 3.0 1000.0))
  (set `self.Min Duration betwen spawns` (`KismetMathLibrary.FClamp` (* (`self.Min Duration betwen spawns`) 0.98) 1.0 1000.0)))

(event `despawn mini bosses`
  ;[1 1 1] despawn ships/booses
  (bind _outactors (`GameplayStatics.GetAllActorsOfClass` "/Game/blueprints/Galaga-proto/Enemy/EnemyBossBP.EnemyBossBP_C"))
  (while (> (`KismetArrayLibrary.Array_Length` _outactors) 1)
    (`self.K2_DestroyActor` (`|GetArrayItem` _outactors))))

(fn `format stage completed text`
  (returns (string :type String))
  (locals (`Stage string` :type String :default "Stage") (`Completed string` :type String :default "Completed") (strings :type "Array of String"))
  (bind _strings (`local.strings`))
  (`KismetArrayLibrary.Array_Add` _strings (`local.Stage string`))
  (`KismetArrayLibrary.Array_Add` _strings (`KismetStringLibrary.Conv_IntToString` (`self.current stage`)))
  (`KismetArrayLibrary.Array_Add` _strings (`local.Completed string`))
  (return (`KismetStringLibrary.JoinStringArray` _strings)))

(fn `Get new ship type`
  (returns (ReturnValue :type "/Game/blueprints/Galaga-proto/Enemy/EnemyTypesEnum Enum") (HitPoints :type Integer) (tier :type Integer))
  (locals (strings :type "Array of String") (`ship type` :type "/Game/blueprints/Galaga-proto/Enemy/EnemyTypesEnum Enum") (`ship tier` :type Integer :default 0))
  (bind _output_get (set `local.ship type` (cast `/Game/blueprints/Galaga-proto/Enemy/EnemyTypesEnum` (`KismetMathLibrary.Conv_IntToByte` (`KismetMathLibrary.RandomInteger` (enumcount `/Game/blueprints/Galaga-proto/Enemy/EnemyTypesEnum`))))))
  (bind _game_tier (`/Game/blueprints/Galaga-proto/GalagaGlobalFunctions.Get game tier` true))
  (bind _output_get_2 (set `local.ship tier` (`KismetMathLibrary.RandomIntegerInRange` 0 _game_tier)))
  (return _output_get (+ (select `/Game/blueprints/Galaga-proto/Enemy/EnemyTypesEnum` _output_get :`NewEnumerator0` 1 :`NewEnumerator1` 2 :`NewEnumerator2` 1) _output_get_2) (+ _output_get_2 1)))

(fn `GetEnemyLane`
  (returns (Lane :type "Float (double-precision)"))
  (locals (startValue :type "Float (double-precision)" :default -10.0) (lastLaneValue :type "Float (double-precision)" :default 9.0) (AllPossibleLanes :type "Array of Float (double-precision)") (index :type "Float (double-precision)") (UsedLanes :type "Array of Float (double-precision)"))
  (bind _allpossiblelanes (`local.AllPossibleLanes`))
  (for _index (range (`KismetMathLibrary.FTrunc` (`local.startValue`)) (+ (`KismetMathLibrary.FTrunc` (`local.lastLaneValue`)) 1))
    (`KismetArrayLibrary.Array_Add` (`local.AllPossibleLanes`) (`KismetMathLibrary.Conv_IntToDouble` _index)))
  (bind _outactors (`GameplayStatics.GetAllActorsOfClass` "/Game/blueprints/Galaga-proto/Enemy/EnemyPlaneBP_2.EnemyPlaneBP_2_C"))
  (for _array_element _outactors
    (`KismetArrayLibrary.Array_RemoveItem` _allpossiblelanes (`/Game/blueprints/Galaga-proto/Enemy/EnemyPlaneBP_2.Lane` _array_element)))
  (`|ExecutionSequence`
    (:`then_1`
      (return (`|GetArrayItem` _allpossiblelanes (`KismetMathLibrary.RandomIntegerInRange` 0 (- (`KismetArrayLibrary.Array_Length` _allpossiblelanes) 1)))))))

(fn `UserConstructionScript`)