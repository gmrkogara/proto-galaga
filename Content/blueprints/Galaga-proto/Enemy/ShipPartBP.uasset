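; ShipPartBP is an enemy ship part in a Galaga prototype, with its own health and timed attacks.
; On BeginPlay it rolls a random enemy type and stage-scaled tier, deriving HP from both plus game stage.
; Hits destroy the damage causer and feed the HUD bonus bar while alive.
; At zero HP it turns black, stops its randomly delayed attack loop, damages its parent actor and awards score.
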(event `self.ReceiveBeginPlay`
  (bind _game_stage (`/Game/blueprints/Galaga-proto/GalagaGameState.Game Stage` (`self.Galaga game state`)))
  ;[1 1 1] begin paly
  (`|ExecutionSequence`
    (:`then_0`
      (bind _galaga_pawn (`/Game/blueprints/Galaga-proto/GalagaGlobalFunctions.Get galaga player pawn`))
      (set `self.galaga player pawn` _galaga_pawn)
      (bind _output (`/Game/blueprints/Galaga-proto/GalagaPlayerPawn.GetHudWidget` _galaga_pawn))
      (set `self.Hud widget` _output)
      (bind _galaga_game_state (`/Game/blueprints/Galaga-proto/GalagaGlobalFunctions.Get galaga game state`))
      (set `self.Galaga game state` _galaga_game_state))
    (:`then_2`
      (set `self.Enemy Type` (cast `/Game/blueprints/Galaga-proto/Enemy/EnemyTypesEnum` (`KismetMathLibrary.Conv_IntToByte` (`KismetMathLibrary.RandomInteger` (enumcount `/Game/blueprints/Galaga-proto/Enemy/EnemyTypesEnum`)))))
      (bind _output_get (set `self.ship tier` (+ (`KismetMathLibrary.RandomIntegerInRange` 0 (`.ReturnValue` (`KismetMathLibrary.FMod` (`KismetMathLibrary.Conv_IntToDouble` _game_stage) 3.0))) 1)))
      (`/Game/blueprints/Galaga-proto/GalagaGlobalFunctions.Set tier indicator` (`self.tier mesh`) _output_get)
      (bind _output_get_2 (set `self.ShipHp` (+ _game_stage _output_get)))
      (set `self.ShipHp` (+ _output_get_2 (select `/Game/blueprints/Galaga-proto/Enemy/EnemyTypesEnum` (`self.Enemy Type`) :`NewEnumerator0` 1 :`NewEnumerator1` 3 :`NewEnumerator2` 2))))))

(event `self.ReceiveAnyDamage`
  (params (Damage :type "Float (single-precision)") (DamageType :type "DamageType Object Reference") (InstigatedBy :type "Controller Object Reference") (DamageCauser :type "Actor Object Reference"))
  (bind _returnvalue (`self.GetParentActor`))
  ;[1 1 1] any damage event
  (if (> (`self.ShipHp`) 0)
    (`|ExecutionSequence`
      (:`then_0`
        (`/Game/blueprints/Galaga-proto/GalagaGameHud.AddValueToBonusBar` (`self.Hud widget`) 3))
      (:`then_1`
        (`self.K2_DestroyActor` DamageCauser :!label _label))
      (:`then_2`
        (bind _output_get (set `self.ShipHp` (- (`self.ShipHp`) (`KismetMathLibrary.FTrunc` Damage))))
        (if (<= _output_get 0)
          (`/Game/blueprints/Galaga-proto/GalagaGlobalFunctions.Set mesh material color` (`self.StaticMesh`) (struct :`A` 1.0))
          (`self.recalculate can shoot bullets`)
          (`/Engine/EditorBlueprintResources/StandardMacros.IsValid` _returnvalue
            (:`Is Valid`
              (`GameplayStatics.ApplyDamage` _returnvalue 1.0)
              (`/Game/blueprints/Galaga-proto/GalagaPlayerPawn.addToPlayerScore` (`self.Galaga player pawn`) 10))))))
    (else
      (goto _label))))

(event `start shooting bullets`
  ;[1 1 1] shooting bullets
  (`KismetSystemLibrary.Delay` (`KismetMathLibrary.RandomFloatInRange` 1.0 5.0) :!label _label_2)
  (if (`self.Can shoot bullets`)
    (`self.Attack`)
    (goto _label_2)))

(event `recalculate can shoot bullets`
  ;[1 1 1] recalculate can shoot bullets
  (set `self.Can shoot bullets` (> (`self.ShipHp`) 0)))

(fn `get bullet starting location`
  (returns (Vector :type "Vector Structure"))
  (return (`SceneComponent.K2_GetComponentLocation` (`self.StaticMesh`))))

(fn `UserConstructionScript`)