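; GalagaGlobalFunctions is a library of shared helpers for the Galaga prototype, covering mesh tinting, player and game state lookup, and tiers.
; Color setters apply a dynamic RGBA material instance to one or all slots, feeding RGB and transparency as parameters.
; Tier derives from GameStage in steps of three, optionally zero-based.
; SetTierIndicator debug-prints and swaps marker meshes, clearing tier 1 and using Tier_1_marker for tier 2.
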(fn `Get galaga game state`
  (returns (`galaga game state` :type "/Game/blueprints/Galaga-proto/GalagaGameState Object Reference"))
  (bind _asgalaga_game_state (cast `/Game/blueprints/Galaga-proto/GalagaGameState` (`GameplayStatics.GetGameState` null)))
  (return _asgalaga_game_state))

(fn `Get galaga player pawn`
  (returns (`Galaga pawn` :type "/Game/blueprints/Galaga-proto/GalagaPlayerPawn Object Reference"))
  (bind _asgalaga_player_pawn (cast `/Game/blueprints/Galaga-proto/GalagaPlayerPawn` (`GameplayStatics.GetPlayerPawn` null)))
  (return _asgalaga_player_pawn))

(fn `Get game tier`
  (params (`zero based?` :type Boolean :default true))
  (returns (`game tier` :type Integer))
  (locals (tier :type Integer))
  (bind _galaga_game_state (`self.Get galaga game state` null))
  (bind _output_get (set `local.tier` (`.ReturnValue` (`KismetMathLibrary.FMod` (`KismetMathLibrary.Conv_IntToDouble` (`/Game/blueprints/Galaga-proto/GalagaGameState.Game Stage` _galaga_game_state)) 3.0))))
  (if (not `zero based?`)
    (`/Engine/EditorBlueprintResources/StandardMacros.IncrementInt` _output_get
      (:`  `
        _)))
  (return (`local.tier`)))

(fn `Set mesh material color`
  (params (`static mesh component` :type "StaticMeshComponent Object Reference") (RGBA :type "LinearColor Structure") (`Material index` :type Integer))
  (bind (_r _g _b _a) (break `LinearColor` RGBA))
  (`PrimitiveComponent.SetMaterial` `static mesh component` `Material index` "/Game/materials/dynamic_RGBA_material_2.dynamic_RGBA_material_2")
  (bind _returnvalue (`PrimitiveComponent.CreateDynamicMaterialInstance` `static mesh component` `Material index` "/Game/materials/dynamic_RGBA_material_2.dynamic_RGBA_material_2" "None"))
  (`MaterialInstanceDynamic.SetScalarParameterValue` _returnvalue "Transparency" _a)
  (`MaterialInstanceDynamic.SetVectorParameterValue` _returnvalue "RBG" (make `LinearColor` _r _g _b 1.0)))

(fn `Set mesh material color for all materials`
  (params (`Static mesh component` :type "StaticMeshComponent Object Reference") (RGBA :type "LinearColor Structure"))
  (for _index (range (+ (`PrimitiveComponent.GetNumMaterials` `Static mesh component`) 1))
    (`self.Set mesh material color` `Static mesh component` RGBA _index)))

(fn `Set tier indicator`
  (params (`tier mesh` :type "StaticMeshComponent Object Reference") (tier :type Integer))
  (locals (stings :type "Array of String"))
  (bind _stings (`local.stings`))
  (`KismetArrayLibrary.Array_Add` _stings (`KismetStringLibrary.Conv_IntToString` tier))
  (`KismetSystemLibrary.PrintString` null (`KismetStringLibrary.JoinStringArray` _stings))
  (switch `int` tier
    (:`1`
      (`StaticMeshComponent.SetStaticMesh` `tier mesh` null))
    (:`2`
      (`StaticMeshComponent.SetStaticMesh` `tier mesh` "/Game/Meshes/Tier_1_marker.Tier_1_marker"))
    (:`3`
      (`StaticMeshComponent.SetStaticMesh` `tier mesh` "/Game/Meshes/tier_3_marker_v2.tier_3_marker_v2"))))