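; Base airplane mesh actor that identifies itself as an enemy and serves as a hittable body for its parent actor.
; When an EnemyBulletBp without the PlayerKiller flag overlaps it, it forwards one point of damage to the parent actor.
; A color function recolors all materials on the static mesh components under its scene root.
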(event `self.ReceiveActorBeginOverlap`
  (params (OtherActor :type "Actor Object Reference"))
  (bind _asenemy_bullet_blueprint (cast `/Game/blueprints/Galaga-proto/Enemy/EnemyBulletBp` OtherActor))
  (if (not (`/Game/blueprints/Galaga-proto/Enemy/EnemyBulletBp.PlayerKiller` _asenemy_bullet_blueprint))
    (`GameplayStatics.ApplyDamage` (`self.GetParentActor`) 1.0 null OtherActor)))

(fn `Are you enemy`
  (returns (`are you ?` :type Boolean))
  (return true))

(fn `set plane material color`
  (params (Color :type "LinearColor Structure"))
  (for _array_element (`SceneComponent.GetChildrenComponents` (`self.DefaultSceneRoot`) true)
    (bind _asstatic_mesh_component (cast `StaticMeshComponent` _array_element))
    (`/Game/blueprints/Galaga-proto/GalagaGlobalFunctions.Set mesh material color for all materials` _asstatic_mesh_component Color)))

(fn `UserConstructionScript`)